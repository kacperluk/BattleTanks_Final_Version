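; Mortar Blueprint that sets up an aimable turret and barrel and a health bar widget for the mortar.
; On BeginPlay it initialises its tank aiming component with the barrel and turret references.
; It then casts the widget component's user widget to HealthBar and sets that widget's Tank reference to itself.
; Tick, overlap and construction script are empty, so no firing or damage logic lives in these graphs.
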(event EventBeginPlay
  (Class|TankAiminngComponent|Initialise (Variables|Default|GetTankAiminng) (Variables|Default|GetTankBarrel) (Variables|Default|GetTankTurret))
  (CallFunction|InitialiseHealthBar))

(event Collision|EventActorBeginOverlap
  (params (OtherActor :type Actor%20Object%20Reference)))

(event EventTick
  (params (DeltaSeconds :type Float%20%28single-precision%29)))

(fn ConstructionScript)

(fn InitialiseHealthBar
  (bind _ashealth_bar (Utilities|Casting|CastToHealthBar (UserInterface|GetUserWidgetObject (Variables|Default|GetWidget))))
  (Variables|/Game/UI/HealthBar.HealthBar_C|Settank _ashealth_bar self))